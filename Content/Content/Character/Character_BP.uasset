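; First-person player character handling movement, look, jump, crouch and a pause menu that pauses the game with UI-only input.
; A camera trace grabs objects with a PhysicsHandle, and Tick holds them in front of the camera until release.
; Left click runs a shorter trace that calls TutorialMessage on actors implementing the Tutorial interface.
; F toggles the LatarkaLight flashlight when MaLatare is true; EquipFlashlight only hides the light.
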(event Custom|Line%20Trace
  (bind _camera (Variables|Default|GetCamera))
  (bind _returnvalue (Transformation|GetWorldLocation _camera))
  ;[1 1 1] Use interface For Doors, Light Switches etc
  (bind (_outhit _returnvalue_2) (Collision|LineTraceByChannel _returnvalue (+ _returnvalue (* (Math|Vector|GetForwardVector _camera) 2e+02)) "TraceTypeQuery1" false 0 "None"))
  (if _returnvalue_2
    (if (Utilities|DoesObjectImplementInterface (.HitActor (Collision|BreakHitResult _outhit)) "/Game/Content/Character/Tutorial.Tutorial_C")
      (Class|Tutorial|Tutorial(Message) (.HitActor (Collision|BreakHitResult _outhit))))))

(event Custom|EquipFlashlight
  ;[1 1 1] Latarka
  (Rendering|SetVisibility (Variables|Default|GetLatarkaLight) false false))

(event EventTick
  (params (DeltaSeconds :type Float%20%28single-precision%29))
  (bind _camera (Variables|Default|GetCamera))
  ;[1 1 1] obiekt podniesiony
  (if (Variables|Default|GetisGrabbing?)
    (Physics|Components|PhysicsHandle|SetTargetLocation (Variables|Default|GetPhysicsHandle) (+ (Transformation|GetWorldLocation _camera) (* (Math|Vector|GetForwardVector (Transformation|GetWorldRotation _camera)) 3e+02)))))

(event Input|ActionEvents|InputActionJump
  (params (Key :type Key%20Structure :default "None"))
  ;[1 1 1] skoki itp
  (:Pressed
    (Character|Jump)))

(event Input|ActionEvents|InputActionCrouch
  (params (Key :type Key%20Structure :default "None"))
  ;[1 1 1] skoki itp
  (:Pressed
    (Character|Crouch))
  (:Released
    (Character|UnCrouch)))

(event Input|ActionEvents|InputActionpodnoszenie
  (params (Key :type Key%20Structure :default "None"))
  (bind _camera (Variables|Default|GetCamera))
  (bind _returnvalue (Transformation|GetWorldLocation _camera))
  ;[1 1 1] grabbing
  (:Pressed
    (bind (_outhit _returnvalue_2) (Collision|LineTraceByChannel _returnvalue (+ _returnvalue (* (Math|Vector|GetForwardVector (Transformation|GetWorldRotation _camera)) 3e+02)) "TraceTypeQuery1" false 0 "None"))
    (if _returnvalue_2
      (Physics|Components|PhysicsHandle|GrabComponentatLocationwithRotation (Variables|Default|GetPhysicsHandle) (.HitComponent (Collision|BreakHitResult _outhit)) "None" (Transformation|GetWorldLocation (.HitComponent (Collision|BreakHitResult _outhit))) "0, 0, 0")
      (Variables|Default|SetisGrabbing? true)))
  (:Released
    (if (Variables|Default|GetisGrabbing?)
      (Physics|Components|PhysicsHandle|ReleaseComponent (Variables|Default|GetPhysicsHandle))
      (Variables|Default|SetisGrabbing? false))))

(event Input|ActionEvents|InputActionPause
  (params (Key :type Key%20Structure :default "None"))
  (bind _returnvalue (Game|GetPlayerController 0))
  ;[1 1 1] Pause Menu
  (:Pressed
    (bind _returnvalue_2 (Game|ConstructObjectfromClass "/Game/Content/UI/PauseMenu.PauseMenu_C"))
    (UserInterface|Viewport|AddtoViewport _returnvalue_2 0)
    (Variables|/Script/Engine.PlayerController|SetbShowMouseCursor _returnvalue true)
    (Input|SetInputModeUIOnly _returnvalue 0 "DoNotLock" false)
    (Game|SetGamePaused true)))

(event Input|AxisEvents|InputAxisForward
  (params (AxisValue :type Float%20%28single-precision%29))
  ;[1 1 1] poruszanie
  (Pawn|Input|AddMovementInput (Math|Vector|GetForwardVector (Variables|Collision|GetCapsuleComponent)) AxisValue false))

(event Input|AxisEvents|InputAxisMoveRight
  (params (AxisValue :type Float%20%28single-precision%29))
  ;[1 1 1] poruszanie
  (Pawn|Input|AddMovementInput (Math|Vector|GetRightVector (Variables|Collision|GetCapsuleComponent)) AxisValue false))

(event Input|AxisEvents|InputAxisTurn
  (params (AxisValue :type Float%20%28single-precision%29))
  ;[1 1 1] camera
  (Pawn|Input|AddControllerYawInput AxisValue))

(event Input|AxisEvents|InputAxisLookUp
  (params (AxisValue :type Float%20%28single-precision%29))
  ;[1 1 1] camera
  (Pawn|Input|AddControllerPitchInput AxisValue))

(event Input|MouseEvents|LeftMouseButton
  (params (Key :type Key%20Structure :default "None"))
  ;[1 1 1] Use interface For Doors, Light Switches etc
  (:Pressed
    (CallFunction|LineTrace)))

(event Input|KeyboardEvents|F
  (params (Key :type Key%20Structure :default "None"))
  ;[1 1 1] Latarka
  (:Pressed
    (if (Variables|Default|GetmaLatare)
      (if (Variables|Default|GetisFlashLightOn)
        (Rendering|SetVisibility (Variables|Default|GetLatarkaLight) false false)
        (Variables|Default|SetisFlashLightOn false)
        (else
          (Rendering|SetVisibility (Variables|Default|GetLatarkaLight) true false)
          (Variables|Default|SetisFlashLightOn true))))))

(fn ConstructionScript)