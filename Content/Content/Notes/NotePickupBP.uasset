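; NotePickupBP is a note that toggles between being read and put down through the Tutorial interface event.
; Picking it up plays a paper sound, shows a widget and hides the cube mesh; putting it down reverses this with the same sound.
; Character_BP overlapping the Cube sets IsCloseEnough, which is never read here.
; Leaving the separate Box clears that flag and automatically puts down a note being read.
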(event OnComponentBeginOverlap(Cube)
  (params (OverlappedComponent :type Primitive%20Component%20Object%20Reference) (OtherActor :type Actor%20Object%20Reference) (OtherComp :type Primitive%20Component%20Object%20Reference) (OtherBodyIndex :type Integer) (bFromSweep :type Boolean) (SweepResult :type Hit%20Result%20Structure%20%28by%20ref%29))
  ;[1 1 1] Box collision if player is reading put down note as walks away
  (Utilities|Casting|CastToCharacter_BP OtherActor)
  (Variables|Default|SetIsCloseEnough? true))

(event OnComponentEndOverlap(Box)
  (params (OverlappedComponent :type Primitive%20Component%20Object%20Reference) (OtherActor :type Actor%20Object%20Reference) (OtherComp :type Primitive%20Component%20Object%20Reference) (OtherBodyIndex :type Integer))
  ;[1 1 1] Box collision if player is reading put down note as walks away
  (Utilities|Casting|CastToCharacter_BP OtherActor)
  (Utilities|FlowControl|Sequence
    (:then_0
      (Variables|Default|SetIsCloseEnough? false)
      (if (Variables|Default|GetIsReading?)
        (CallFunction|PutdownNOte)))))

(event Custom|Putdown%20NOte
  ;[1 1 1] Putdown Note event
  (Audio|PlaySoundatLocation "/Game/Content/Notes/paper-245786.paper-245786" (Transformation|GetWorldLocation (Variables|Default|GetCube)) "0, 0, 0" 1.0 1.0 0.0 0 0 0 0)
  (Widget|RemovefromParent (stale Custom|PickuoNote _returnvalue))
  (Rendering|SetVisibility (Variables|Default|GetCube) true false)
  (Variables|Default|SetIsReading? false))

(event Custom|Toggle%20Pickup
  ;[1 1 1] Toggle Event Pickup and putdown
  (if (Variables|Default|GetIsReading?)
    (CallFunction|PutdownNOte)
    (else
      (CallFunction|PickuoNote))))

(event Custom|PickuoNote
  ;[1 1 1] Pickup Note event
  (Audio|PlaySoundatLocation "/Game/Content/Notes/paper-245786.paper-245786" (Transformation|GetWorldLocation (Variables|Default|GetCube)) "0, 0, 0" 1.0 1.0 0.0 0 0 0 0)
  (bind _returnvalue (UserInterface|CreateWidget (Variables|Default|GetClass)))
  (UserInterface|Viewport|AddtoViewport _returnvalue 0)
  (Rendering|SetVisibility (Variables|Default|GetCube) false false)
  (Variables|Default|SetIsReading? true))

(event EventTutorial
  (params (Actor :type Actor%20Object%20Reference))
  ;[1 1 1] Toggle Pickup BP Interface
  (CallFunction|TogglePickup))

(fn ConstructionScript)