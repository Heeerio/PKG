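; Light puzzle checker that tests whether the puzzle pieces show the right color code and, when solved, signals a linked door.
; The Tutorial event compares each piece's ColorIndex with ColorCode at the same index, stopping at the first mismatch.
; A match passes through a DoOnce to call the door's Tutorial interface message.
; On a mismatch it loops the pieces without effect, as the color-reset nodes are disconnected.
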(event EventTutorial
  (params (Actor :type Actor%20Object%20Reference))
  (Variables|Default|SetIsCorrect? true)
  (bind (_array_element _array_index) (Utilities|Array|ForEachLoopwithBreak (Variables|Default|GetPuzzlePieces) :!label _label)
    (:LoopBody
      (if (!= (Variables|/Game/Content/LightPuzzle/BP_Light_PuzzlePice.BP_Light_PuzzlePice_C|GetColorIndex _array_element) (Utilities|Array|Get(acopy) (Variables|Default|GetColorCode) _array_index))
        (Variables|Default|SetIsCorrect? false)
        (goto _label Break)))
    (:Completed
      (if (Variables|Default|GetIsCorrect?)
        (Utilities|FlowControl|DoOnce false
          (:Completed
            (bind _doortoopen (Variables|Default|GetDoorToOpen)
              (:then
                (if (Utilities|DoesObjectImplementInterface _doortoopen "/Game/Content/Character/Tutorial.Tutorial_C")
                  (Class|Tutorial|Tutorial(Message) _doortoopen self)))
              (:else))))
        (else
          (for _array_element_2 (Variables|Default|GetPuzzlePieces)
            _))))))

(fn ConstructionScript)